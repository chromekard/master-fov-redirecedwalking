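; BP_Rotation_Character is a character Blueprint that continually replays a yaw rotation.
; On BeginPlay, Timeline_Rotation drives a lerp from zero to MaxRotation, which sets the absolute actor yaw with pitch and roll held at zero.
; When the timeline finishes, it waits briefly and plays from the start, so each cycle begins again at zero yaw.
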(event `self.ReceiveBeginPlay`
  (`parent.ReceiveBeginPlay`)
  (bind (_direction _alpha) (`Timeline|Timeline_Rotation` :!label _label)
    (:`Update`
      (`self.K2_SetActorRotation` (`KismetMathLibrary.MakeRotator` 0.0 0.0 (`KismetMathLibrary.Lerp` 0.0 (`self.MaxRotation`) _alpha))))
    (:`Finished`
      (`KismetSystemLibrary.Delay` 2.0)
      (goto _label :!via `PlayFromStart`))))

(event `self.ReceiveTick`
  (params (DeltaSeconds :type "Float (single-precision)"))
  (`parent.ReceiveTick` DeltaSeconds))

(fn `UserConstructionScript`
  (`parent.UserConstructionScript`))