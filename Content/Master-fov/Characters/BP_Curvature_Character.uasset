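; Self-driving character that repeatedly walks a curved path without player input.
; On BeginPlay, Timeline_Curvature blends a yaw offset up to MaxRotation from the InitialState rotation, turning the actor and feeding half-scale movement input along that heading.
; When the timeline finishes, it waits briefly, resets the transform to InitialState and replays.
; InitialState is only read here, never assigned.
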(event `self.ReceiveBeginPlay`
  (`parent.ReceiveBeginPlay`)
  (bind (_direction _alpha) (`Timeline|Timeline_Curvature` :!label _label)
    (:`Update`
      (bind _returnvalue (`KismetMathLibrary.Lerp` 0.0 (`self.MaxRotation`) _alpha))
      (`self.K2_SetActorRotation` (`KismetMathLibrary.ComposeRotators` (.rotation (`self.InitialState`)) (`KismetMathLibrary.MakeRotator` 0.0 0.0 _returnvalue)))
      (`self.AddMovementInput` (`KismetMathLibrary.GetForwardVector` (`KismetMathLibrary.MakeRotator` (.roll (.rotation (`self.InitialState`))) (.pitch (.rotation (`self.InitialState`))) (+ (.yaw (.rotation (`self.InitialState`))) _returnvalue))) 0.5))
    (:`Finished`
      (`KismetSystemLibrary.Delay` 2.0)
      (`self.K2_SetActorTransform` (`self.InitialState`))
      (goto _label :!via `PlayFromStart`))))

(fn `UserConstructionScript`
  (`parent.UserConstructionScript`))