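; BP_Translation_Character is a character Blueprint that repeatedly drives itself along its forward direction, then resets.
; On BeginPlay, after the parent call, a timeline feeds its Alpha curve, scaled by Gain, into AddMovementInput along the actor's forward vector.
; When the timeline finishes, the character waits briefly, snaps back to the InitialState transform and replays the timeline from the start, forming an endless loop.
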(event `self.ReceiveBeginPlay`
  (`parent.ReceiveBeginPlay`)
  (bind (_direction _alpha) (`Timeline|Timeline_Translation` :!label _label)
    (:`Update`
      (`self.AddMovementInput` (`KismetMathLibrary.GetForwardVector` (`self.K2_GetActorRotation`)) (* _alpha (`self.Gain`))))
    (:`Finished`
      (`KismetSystemLibrary.Delay` 2.0)
      (`self.K2_SetActorTransform` (`self.InitialState`))
      (goto _label :!via `PlayFromStart`))))

(fn `UserConstructionScript`
  (`parent.UserConstructionScript`))