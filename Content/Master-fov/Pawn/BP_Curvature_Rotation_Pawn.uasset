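; Pawn that tests a curvature rotation gain, as used in redirected walking, with keys moving and turning Sphere1 inside it.
; Each Tick measures Sphere1's relative movement and yaws the actor in proportion to distance times Gain.
; An added location offset makes the actor pivot around the sphere's world position instead of its own origin.
; E applies the same pivot by a set Angle, and debug prints report deltas and transforms.
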(event `self.ReceiveBeginPlay`
  (bind _relativelocation (`SceneComponent.RelativeLocation` (`self.Sphere1`)))
  (set `self.CurPosReal` _relativelocation)
  (set `self.PrevPosReal` _relativelocation))

(event `self.ReceiveTick`
  (params (DeltaSeconds :type "Float (single-precision)"))
  (bind _returnvalue (`KismetMathLibrary.VSize` (`self.DeltaPos`)))
  (bind _returnvalue_2 (- (`self.K2_GetActorLocation`) (`SceneComponent.K2_GetComponentLocation` (`self.Sphere1`))))
  (bind _returnvalue_3 (* (/ _returnvalue 500.0) (`self.Gain`)))
  (bind _output_get (set `self.CurPosReal` (`SceneComponent.RelativeLocation` (`self.Sphere1`))))
  (set `self.DeltaPos` (- (`self.CurPosReal`) (`self.PrevPosReal`)))
  (set `self.PrevPosReal` _output_get)
  (if (and (!= (`self.Gain`) 0.0) (!= (`self.DeltaPos`) (0.0 0.0 0.0)))
    (`KismetSystemLibrary.PrintString` (`KismetStringLibrary.Concat_StrStr` "Delta Length: " (`KismetStringLibrary.Conv_DoubleToString` _returnvalue)))
    (`KismetSystemLibrary.PrintString` (`KismetStringLibrary.Concat_StrStr` "Angle: " (`KismetStringLibrary.Conv_DoubleToString` _returnvalue_3)))
    (`self.K2_AddActorWorldTransform` (`KismetMathLibrary.MakeTransform` (- (`KismetMathLibrary.RotateAngleAxis` _returnvalue_2 _returnvalue_3 (0.0 0.0 1.0)) _returnvalue_2) (`KismetMathLibrary.MakeRotator` 0.0 0.0 _returnvalue_3)) false true)))

(event `Key|W`
  (params (Key :type "Key Structure"))
  (:`Pressed`
    (`SceneComponent.K2_AddLocalOffset` (`self.Sphere1`) (500.0 0.0 0.0) false false)
    (`KismetSystemLibrary.PrintString` (`KismetStringLibrary.Concat_StrStr` "Actor location: " (`KismetStringLibrary.Conv_VectorToString` (`self.K2_GetActorLocation`))) :!label _label)
    (`KismetSystemLibrary.PrintString` (`KismetStringLibrary.Concat_StrStr` "Actor rotation: " (`KismetStringLibrary.Conv_RotatorToString` (`self.K2_GetActorRotation`))))
    (`KismetSystemLibrary.PrintString` (`KismetStringLibrary.Concat_StrStr` "Sphere location: " (`KismetStringLibrary.Conv_VectorToString` (`SceneComponent.RelativeLocation` (`self.Sphere1`)))))
    (`KismetSystemLibrary.PrintString` (`KismetStringLibrary.Concat_StrStr` "Sphere Rotation: " (`KismetStringLibrary.Conv_RotatorToString` (`SceneComponent.RelativeRotation` (`self.Sphere1`)))))))

(event `Key|E`
  (params (Key :type "Key Structure"))
  (bind _angle (`self.Angle`))
  (bind _returnvalue (- (`self.K2_GetActorLocation`) (`SceneComponent.K2_GetComponentLocation` (`self.Sphere1`))))
  (:`Pressed`
    (`self.K2_AddActorWorldTransform` (`KismetMathLibrary.MakeTransform` (- (`KismetMathLibrary.RotateAngleAxis` _returnvalue _angle (0.0 0.0 1.0)) _returnvalue) (`KismetMathLibrary.MakeRotator` 0.0 0.0 _angle)) false true)))

(event `Key|S`
  (params (Key :type "Key Structure"))
  (:`Pressed`
    (`SceneComponent.K2_AddLocalOffset` (`self.Sphere1`) (-10.0 0.0 0.0) false false)
    (goto _label)))

(event `Key|A`
  (params (Key :type "Key Structure"))
  (:`Pressed`
    (`SceneComponent.K2_AddLocalOffset` (`self.Sphere1`) (0.0 10.0 0.0) false false)
    (goto _label)))

(event `Key|Q`
  (params (Key :type "Key Structure"))
  (:`Pressed`
    (`SceneComponent.K2_AddRelativeRotation` (`self.Sphere1`) (struct :`Yaw` 45.0) false false)))

(event `Key|D`
  (params (Key :type "Key Structure"))
  (:`Pressed`
    (`SceneComponent.K2_AddLocalOffset` (`self.Sphere1`) (0.0 -10.0 0.0) false false)
    (goto _label)))

(fn `UserConstructionScript`)