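; Game mode that sequences a VR experiment through Tutorial, Measurement, Staging and Threshold stages, then quits the game.
; Initialization reads the experiment type (Rotation, Translation or Curvature) from the GameInstance to pick Staging and Threshold pawn classes; its FOV check has no effect.
; NextStage honors the GameInstance's skip flags.
; Each stage spawns its own pawn, which the player controller possesses and whose done event triggers the next stage.
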(event `Event_Initialize`
  ;[1 1 1] Setup
  (bind _asbp_container_game_instance (cast `/Game/Master-fov/Blueprints/GameInstance/BP_Container_GameInstance` (`GameplayStatics.GetGameInstance`)))
  (switch `/Game/Master-fov/Enum/ExperimentType` (`/Game/Master-fov/Blueprints/GameInstance/BP_Container_GameInstance.Experiment_Type` _asbp_container_game_instance)
    (:`NewEnumerator0`
      (set `self.StagingClass` "/Game/Master-fov/Pawn/GainPawns/StagingPawns/VR_Staging_Rotation_Pawn.VR_Staging_Rotation_Pawn_C")
      (set `self.ThresholdClass` "/Game/Master-fov/Pawn/GainPawns/ThresholdPawns/VR_Rotation_Pawn.VR_Rotation_Pawn_C"))
    (:`NewEnumerator1`
      (set `self.StagingClass` "/Game/Master-fov/Pawn/GainPawns/StagingPawns/VR_Staging_TranslationPawn.VR_Staging_TranslationPawn_C")
      (set `self.ThresholdClass` "/Game/Master-fov/Pawn/GainPawns/ThresholdPawns/VR_Translation_Pawn.VR_Translation_Pawn_C"))
    (:`NewEnumerator2`
      (set `self.StagingClass` "/Game/Master-fov/Pawn/GainPawns/StagingPawns/VR_Staging_Curvature_Pawn.VR_Staging_Curvature_Pawn_C")
      (set `self.ThresholdClass` "/Game/Master-fov/Pawn/GainPawns/ThresholdPawns/VR_Curvature_Pawn.VR_Curvature_Pawn_C")))
  (if (== (`/Game/Master-fov/Blueprints/GameInstance/BP_Container_GameInstance.FOV` _asbp_container_game_instance) 40)
    _
    (else
      _))
  (`self.Event_NextExperiment`))

(event `Event_NextExperiment`
  (bind _nextstage (`self.NextStage`))
  ;[1 1 1] Next stage
  (if (`|EnumEquality` "NewEnumerator3" _nextstage)
    ;[1 1 1] Do something
    (`KismetSystemLibrary.QuitGame` null "Quit")
    (else
      (bind _output_get (set `self.CurStage` _nextstage))
      (bind _pawn (`self.CreateStagePawn` _output_get))
      (`Controller.Possess` (`GameplayStatics.GetPlayerController` 0) _pawn)
      (`/Game/Master-fov/Pawn/GainPawns/VR_Gain_Base_Pawn.BindDoneEvent` _pawn (delegate `Event_NextExperiment`)))))

(fn `CreateStagePawn`
  (params (Stage :type "/Game/Master-fov/Enum/ExperimentStages Enum" :default "NewEnumerator3"))
  (returns (Pawn :type "/Game/Master-fov/Pawn/GainPawns/VR_Gain_Base_Pawn Object Reference"))
  (switch `/Game/Master-fov/Enum/ExperimentStages` Stage
    (:`NewEnumerator3`
      (return null))
    (:`NewEnumerator4`
      (bind _returnvalue (`|SpawnActorFromClass` "/Game/Master-fov/Pawn/VR_Tutorial_Pawn.VR_Tutorial_Pawn_C" (`self.TurorialPoint`) "AlwaysSpawn" "OverrideRootScale" (`GameplayStatics.GetPlayerController` 0) null))
      (return _returnvalue))
    (:`NewEnumerator0`
      (bind _returnvalue_2 (`|SpawnActorFromClass` "/Game/Master-fov/Pawn/GainPawns/VR_Measurement_Pawn.VR_Measurement_Pawn_C" (`self.MeasurementPoint`) "AlwaysSpawn" "OverrideRootScale" (`GameplayStatics.GetPlayerController` 0) null))
      (return _returnvalue_2))
    (:`NewEnumerator1`
      (bind _returnvalue_3 (`|SpawnActorFromClass` (`self.StagingClass`) (`self.StagingPoint`) "AlwaysSpawn" "OverrideRootScale" (`GameplayStatics.GetPlayerController` 0) null))
      (return _returnvalue_3))
    (:`NewEnumerator2`
      (bind _returnvalue_4 (`|SpawnActorFromClass` (`self.ThresholdClass`) (`self.ThresholdPoint`) "AlwaysSpawn" "OverrideRootScale" (`GameplayStatics.GetPlayerController` 0) null))
      (return _returnvalue_4))))

(fn `NextStage`
  (returns (NextStage :type "/Game/Master-fov/Enum/ExperimentStages Enum"))
  (bind _asbp_container_game_instance (cast `/Game/Master-fov/Blueprints/GameInstance/BP_Container_GameInstance` (`GameplayStatics.GetGameInstance`))
    (:`then`
      (switch `/Game/Master-fov/Enum/ExperimentStages` (`self.CurStage`)
        (:`NewEnumerator3`
          (if (not (`/Game/Master-fov/Blueprints/GameInstance/BP_Container_GameInstance.SkipTutorial` _asbp_container_game_instance))
            (return "NewEnumerator4")
            (else
              (if (not (`/Game/Master-fov/Blueprints/GameInstance/BP_Container_GameInstance.SkipMeasurement` _asbp_container_game_instance)) :!label _label
                _
                (else
                  (if (not (`/Game/Master-fov/Blueprints/GameInstance/BP_Container_GameInstance.SkipStaging` _asbp_container_game_instance)) :!label _label_2
                    (return "NewEnumerator1")
                    (else
                      (if (not (`/Game/Master-fov/Blueprints/GameInstance/BP_Container_GameInstance.SkipThreshold` _asbp_container_game_instance)) :!label _label_3
                        (return "NewEnumerator2")
                        (else
                          (return "NewEnumerator3"))))))))))
        (:`NewEnumerator4`
          (goto _label))
        (:`NewEnumerator0`
          (goto _label_2))
        (:`NewEnumerator1`
          (goto _label_3))
        (:`NewEnumerator2`
          (return "NewEnumerator3")))
      (return "NewEnumerator0"))
    (:`CastFailed`
      (switch `/Game/Master-fov/Enum/ExperimentStages` (`self.CurStage`)
        (:`NewEnumerator3`
          (return "NewEnumerator4"))
        (:`NewEnumerator4`
          (return "NewEnumerator0"))
        (:`NewEnumerator0`
          (return "NewEnumerator1"))
        (:`NewEnumerator1`
          (return "NewEnumerator2"))
        (:`NewEnumerator2`
          (return "NewEnumerator3"))))))

(fn `UserConstructionScript`)