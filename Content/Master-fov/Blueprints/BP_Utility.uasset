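; BP_Utility provides two stateless vector math helpers for working with directions.
; FlattenDir3D zeroes a vector's Z component without renormalizing it.
; GetSignedAngle returns the degrees between two directions from the normalized dot product, signed by the Z of their cross product.
; It does not flatten its inputs, and returns zero whenever that Z is zero, including for exactly opposite directions.
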(fn `FlattenDir3D`
  (params (Vector :type "Vector Structure"))
  (returns (FlatVector :type "Vector Structure"))
  (return (`KismetMathLibrary.MakeVector` (.x Vector) (.y Vector))))

(fn `GetSignedAngle`
  (params (PrevDir :type "Vector Structure") (CurDir :type "Vector Structure"))
  (returns (SignedAngle :type "Float (double-precision)"))
  (return (* (`KismetMathLibrary.SignOfFloat` (.z (`KismetMathLibrary.Cross_VectorVector` PrevDir CurDir))) (`KismetMathLibrary.DegAcos` (`KismetMathLibrary.Dot_VectorVector` (`KismetMathLibrary.Normal` PrevDir) (`KismetMathLibrary.Normal` CurDir))))))