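; Game Instance that holds participant info and gain-threshold answers for an FOV experiment and saves them as comma-separated files.
; AddResults, gated by an Accepting flag, logs each answer in order and sums it per gain in a map pre-seeded by InitializeThresholdMap.
; Shutdown, unless already saved or purged, writes a per-user file and appends to shared summaries, named by experiment type and FOV.
; PrintTrackingData separately exports position/rotation event logs.
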(event `self.ReceiveShutdown`
  (if (`self.bSaved`)
    _
    (elif (not (`self.bPurge`))
      (`self.PrintToFile`))))

(fn `AddResults`
  (params (Gain :type "Float (double-precision)") (Results :type Integer))
  (returns (Success :type Boolean))
  (bind (_value _returnvalue) (`BlueprintMapLibrary.Map_Find` (`self.MappedThresholdAnswers`) Gain))
  (if (`self.bAccepting`)
    (set `self.bAccepting` false)
    (`KismetArrayLibrary.Array_Add` (`self.SeriedThresholdAnswers`) (make `/Game/Master-fov/Struct/GainResults` Gain Results))
    (if _returnvalue
      (`BlueprintMapLibrary.Map_Add` (`self.MappedThresholdAnswers`) Gain (+ _value Results))
      (return true)
      (else
        (`BlueprintMapLibrary.Map_Add` (`self.MappedThresholdAnswers`) Gain Results)
        (return true)))
    (else
      (return false))))

(fn `InitializeThresholdMap`
  (params (`Ordered Key Set` :type "Set of Float (double-precision)"))
  (bind _result (`BlueprintSetLibrary.Set_ToArray` `Ordered Key Set`))
  (for _array_element _result
    (`BlueprintMapLibrary.Map_Add` (`self.MappedThresholdAnswers`) _array_element))
  (return))

(fn `MappedThresholdsToString`
  (params (WithHeader :type Boolean))
  (returns (Results :type String))
  (locals (Text :type String))
  (if WithHeader
    ;[1 1 1] Create Header
    (set `local.Text` "UserId, ")
    (bind _keys (`BlueprintMapLibrary.Map_Keys` (`self.MappedThresholdAnswers`)))
    (for _array_element _keys
      (set `local.Text` (`KismetStringLibrary.Concat_StrStr` (`local.Text`) (`KismetStringLibrary.Conv_DoubleToString` _array_element) ", ")))
    (set `local.Text` (`KismetStringLibrary.Concat_StrStr` (`local.Text`) " \n")))
  (set `local.Text` (`KismetStringLibrary.Concat_StrStr` (`local.Text`) (`self.UserId`) ", "))
  (bind _values (`BlueprintMapLibrary.Map_Values` (`self.MappedThresholdAnswers`)))
  (for _array_element_2 _values
    (set `local.Text` (`KismetStringLibrary.Concat_StrStr` (`local.Text`) (`KismetStringLibrary.Conv_IntToString` _array_element_2) ", ")))
  (return (`local.Text`)))

(fn `PrintToFile`
  (bind _returnvalue (`KismetStringLibrary.Concat_StrStr` (`self.UserInfoToString` true) " \n" (`self.MappedThresholdsToString` true) " \n" (`self.SeriedThresholdsToString` true)))
  (bind _returnvalue_2 (`KismetStringLibrary.Concat_StrStr` (`|GetEnumeratorNameAsString` (`self.Experiment_Type`)) "_" (`KismetStringLibrary.Conv_IntToString` (`self.FOV`)) "_" (`self.ThresholdSummaryFileName`)))
  (bind _returnvalue_3 (`KismetStringLibrary.Concat_StrStr` (`|GetEnumeratorNameAsString` (`self.Experiment_Type`)) "_" (`KismetStringLibrary.Conv_IntToString` (`self.FOV`)) "_" (`self.UserSummaryFileName`)))
  (bind _returnvalue_4 (`KismetStringLibrary.Concat_StrStr` (`|GetEnumeratorNameAsString` (`self.Experiment_Type`)) "_" (`KismetStringLibrary.Conv_IntToString` (`self.FOV`)) "_" (`self.UserId`) (`self.SubjectFileEnding`)))
  (bind _returnvalue_5 (`KismetStringLibrary.Concat_StrStr` (`self.SaveDir`) _returnvalue_4))
  (bind _returnvalue_6 (`KismetStringLibrary.Concat_StrStr` (`self.SaveDir`) _returnvalue_2))
  (bind _returnvalue_7 (`KismetStringLibrary.Concat_StrStr` (`self.SaveDir`) _returnvalue_3))
  (`|ExecutionSequence`
    (:`then_0`
      ;[1 1 1] Participant data
      (if (`UtilityFunctionLibrary.DoesFileExist` _returnvalue_5)
        (if (`self.bOverrideExisting`)
          (`UtilityFunctionLibrary.FileIO__SaveStringTextToFile` (`self.SaveDir`) _returnvalue_4 _returnvalue true :!label _label)
          (else
            (bind (_savetexta _returnvalue_8) (`UtilityFunctionLibrary.FileIO__LoadStringFromFile` false _returnvalue_5))
            (if _returnvalue_8
              (`UtilityFunctionLibrary.FileIO__SaveStringTextToFile` (`self.SaveDir`) _returnvalue_4 (`KismetStringLibrary.Concat_StrStr` _savetexta " \n" _returnvalue) true)
              (else
                (`KismetSystemLibrary.PrintString` "Failed to load user id file to string")
                (`KismetSystemLibrary.PrintString` (`KismetStringLibrary.Concat_StrStr` "FilePath: " _returnvalue_5))))))
        (else
          (goto _label))))
    (:`then_1`
      ;[1 1 1] Sumerized paticipant data
      (if (`UtilityFunctionLibrary.DoesFileExist` _returnvalue_7)
        (bind (_savetexta_2 _returnvalue_9) (`UtilityFunctionLibrary.FileIO__LoadStringFromFile` false _returnvalue_7))
        (if _returnvalue_9
          (bind _returnvalue_10 (`UtilityFunctionLibrary.FileIO__SaveStringTextToFile` (`self.SaveDir`) _returnvalue_3 (`KismetStringLibrary.Concat_StrStr` _savetexta_2 " \n" (`self.UserInfoToString` false)) true))
          (if (not _returnvalue_10)
            (`KismetSystemLibrary.PrintString` "Failed to save  summary file to string"))
          (else
            (`KismetSystemLibrary.PrintString` "Failed to load user summary file to string")))
        (else
          (`UtilityFunctionLibrary.FileIO__SaveStringTextToFile` (`self.SaveDir`) _returnvalue_3 (`self.UserInfoToString` true) true))))
    (:`then_2`
      ;[1 1 1] Summerized Threhsold data
      (if (`UtilityFunctionLibrary.DoesFileExist` _returnvalue_6)
        (bind (_savetexta_3 _returnvalue_11) (`UtilityFunctionLibrary.FileIO__LoadStringFromFile` false _returnvalue_6))
        (if _returnvalue_11
          (`UtilityFunctionLibrary.FileIO__SaveStringTextToFile` (`self.SaveDir`) _returnvalue_2 (`KismetStringLibrary.Concat_StrStr` _savetexta_3 " \n" (`self.MappedThresholdsToString` false)) true)
          (else
            (`KismetSystemLibrary.PrintString` "Failed to load threshold summary file to string")))
        (else
          (`UtilityFunctionLibrary.FileIO__SaveStringTextToFile` (`self.SaveDir`) _returnvalue_2 (`self.MappedThresholdsToString` true) true))))
    (:`then_3`
      (set `self.bSaved` true))))

(fn `PrintTrackingData`
  (params (type :type String) (Array :type "Array of /Game/Master-fov/Struct/TrackingData Structure (by ref)") (FileIteration :type Integer))
  (returns (ReturnValue :type Boolean))
  (bind _returnvalue (`UtilityFunctionLibrary.FileIO__SaveStringTextToFile` (`self.SaveDir`) (`KismetStringLibrary.Concat_StrStr` (`|GetEnumeratorNameAsString` (`self.Experiment_Type`)) "_" (`KismetStringLibrary.Conv_IntToString` (`self.FOV`)) "_" (`self.UserId`) "_" type (`KismetStringLibrary.Conv_IntToString` FileIteration) "_" (`self.TrackingDataFileEnding`)) (`self.TrackingToString` true Array) (`self.bOverrideExisting`)))
  (return _returnvalue))

(fn `SeriedThresholdsToString`
  (params (WithHeader :type Boolean))
  (returns (String :type String))
  (locals (Text :type String))
  (if WithHeader
    (set `local.Text` "Gain, Answer, \n"))
  (for _array_element (`self.SeriedThresholdAnswers`)
    (bind (_gain _answer) (break `/Game/Master-fov/Struct/GainResults` _array_element))
    (set `local.Text` (`KismetStringLibrary.Concat_StrStr` (`local.Text`) (`KismetStringLibrary.Conv_DoubleToString` _gain) ", " (`KismetStringLibrary.Conv_IntToString` _answer) ", \n")))
  (return (`local.Text`)))

(fn `SortMappedThresholds`
  (params (Array :type "Array of /Game/Master-fov/Struct/GainResults Structure"))
  (returns (SortedArray :type "Array of /Game/Master-fov/Struct/GainResults Structure"))
  (locals (TempArray :type "Array of /Game/Master-fov/Struct/GainResults Structure") (Temp :type "/Game/Master-fov/Struct/GainResults Structure"))
  (bind _output_get (set `local.TempArray` Array))
  (bind _returnvalue (`KismetArrayLibrary.Array_Length` _output_get))
  (for _ (range (+ _returnvalue 1))
    (for _index (range (+ (- _returnvalue 2) 1))
      ;[1 1 1] Swap indexes
      (if (> (`.Gain_4_DE7032F949E1D361072EFAA87EDB2072` (break `/Game/Master-fov/Struct/GainResults` (`|GetArrayItem` (`local.TempArray`) _index))) (`.Gain_4_DE7032F949E1D361072EFAA87EDB2072` (break `/Game/Master-fov/Struct/GainResults` (`|GetArrayItem` (`local.TempArray`) (+ _index 1)))))
        (set `local.Temp` (`|GetArrayItem` (`local.TempArray`) _index))
        (`KismetArrayLibrary.Array_Set` (`local.TempArray`) _index (`|GetArrayItem` (`local.TempArray`) (+ _index 1)))
        (`KismetArrayLibrary.Array_Set` (`local.TempArray`) (+ _index 1) (`local.Temp`)))))
  (return (`local.TempArray`)))

(fn `TrackingToString`
  (params (WithHeader :type Boolean) (Array :type "Array of /Game/Master-fov/Struct/TrackingData Structure"))
  (returns (String :type String))
  (locals (Text :type String))
  (if WithHeader
    (set `local.Text` "Event, x, y, z, roll, pitch, yaw, \n"))
  (for _array_element Array
    (bind (_eventtype _position _rotation) (break `/Game/Master-fov/Struct/TrackingData` _array_element))
    (set `local.Text` (`KismetStringLibrary.Concat_StrStr` (`local.Text`) _eventtype ", " (`KismetStringLibrary.Conv_DoubleToString` (.x _position)) "," (`KismetStringLibrary.Conv_DoubleToString` (.y _position)) "," (`KismetStringLibrary.Conv_DoubleToString` (.z _position)) "," (`KismetStringLibrary.Conv_DoubleToString` (.roll _rotation)) "," (`KismetStringLibrary.Conv_DoubleToString` (.pitch _rotation)) "," (`KismetStringLibrary.Conv_DoubleToString` (.yaw _rotation)) ", \n")))
  (return (`local.Text`)))

(fn `UserInfoToString`
  (params (bWithHeader :type Boolean))
  (returns (Info :type String))
  (bind _returnvalue (`KismetStringLibrary.Concat_StrStr` (`self.UserId`) ", " (`KismetStringLibrary.Conv_DoubleToString` (`self.Height`)) ", " (`KismetStringLibrary.Conv_DoubleToString` (`self.Gait`)) ", " (`KismetStringLibrary.Conv_DoubleToString` (`self.DTPositive`)) ", " (`KismetStringLibrary.Conv_DoubleToString` (`self.MaxGainPositive`)) ", " (`KismetStringLibrary.Conv_DoubleToString` (`self.DTNegative`)) ", " (`KismetStringLibrary.Conv_DoubleToString` (`self.MaxGainNegative`))))
  (if bWithHeader
    (return (`KismetStringLibrary.Concat_StrStr` "UserID, Height, Gait, DTPositive, MxGainPos, DTNegative, MxGainNeg, \n" _returnvalue))
    (else
      (return _returnvalue))))