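; BP_Auto_Cannon_Actor is an automatic cannon that spawns bombs and displays its own score.
; While enabled, Tick spawns a BP_Bomb_Actor at the muzzle at random intervals, and a restarting timeline applies small yaw offsets to turn the cannon.
; Each bomb's explode-pawn event lowers or raises the score by its Bomb flag and updates the number widget.
; SetEnabled switches both firing and animation.
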(event `Event_Animate`
  (params (Enabled :type Boolean))
  (if Enabled
    (bind (_direction _delta) (`Timeline|Timeline_Delta` :!label _label)
      (:`Update`
        (`self.K2_AddActorWorldRotation` (`KismetMathLibrary.MakeRotator` 0.0 0.0 (`KismetMathLibrary.Lerp` -0.2 0.2 _delta))))
      (:`Finished`
        (goto _label :!via `PlayFromStart`)))
    (else
      (goto _label :!via `Stop`))))

(event `self.ReceiveBeginPlay`
  (set `self.Limit` (`KismetMathLibrary.RandomFloatInRange` 1.0 5.0))
  (bind _asbp_number_widget (cast `/Game/Master-fov/Widgets/3DWidgets/BP_Number_Widget` (`WidgetComponent.GetUserWidgetObject` (`self.Widget`))))
  (`TextBlock.SetText` (`/Game/Master-fov/Widgets/3DWidgets/BP_Number_Widget.TextBlock_Number` _asbp_number_widget) (`KismetTextLibrary.Conv_IntToText` (`self.Score`)))
  (`self.Event_Animate` (`self.bEnabled`)))

(event `self.ReceiveTick`
  (params (DeltaSeconds :type "Float (single-precision)"))
  (if (`self.bEnabled`)
    (set `self.Agrigate` (+ DeltaSeconds (`self.Agrigate`)))
    (if (> (`self.Agrigate`) (`self.Limit`))
      (set `self.Agrigate` 0.0)
      (set `self.Limit` (`KismetMathLibrary.RandomFloatInRange` 1.0 5.0))
      (bind _returnvalue (`|SpawnActorFromClass` "/Game/Master-fov/Blueprints/Objects/BP_Bomb_Actor.BP_Bomb_Actor_C" (`KismetMathLibrary.MakeTransform` (.location (`SceneComponent.K2_GetComponentToWorld` (`self.Muzzle`))) (.rotation (`SceneComponent.K2_GetComponentToWorld` (`self.Muzzle`))) (.scale (`SceneComponent.K2_GetComponentToWorld` (`self.Muzzle`)))) "AlwaysSpawn" "OverrideRootScale" null null))
      (add `/Game/Master-fov/Blueprints/Objects/BP_Bomb_Actor.Event_ExplodePawn` _returnvalue (delegate `Event_Hit`)))))

(event `Event_Hit`
  (params (bomb :type Boolean))
  (if bomb
    (`/Engine/EditorBlueprintResources/StandardMacros.DecrementInt` (`self.Score`)
      (:`  `
        _))
    (else
      (`/Engine/EditorBlueprintResources/StandardMacros.IncrementInt` (`self.Score`)
        (:`  `
          _))))
  (bind _asbp_number_widget (cast `/Game/Master-fov/Widgets/3DWidgets/BP_Number_Widget` (`WidgetComponent.GetUserWidgetObject` (`self.Widget`))))
  (`TextBlock.SetText` (`/Game/Master-fov/Widgets/3DWidgets/BP_Number_Widget.TextBlock_Number` _asbp_number_widget) (`KismetTextLibrary.Conv_IntToText` (`self.Score`))))

(fn `SetEnabled`
  (params (Enabled :type Boolean))
  (bind _output_get (set `self.bEnabled` Enabled))
  (`self.Event_Animate` _output_get)
  (return))

(fn `UserConstructionScript`)