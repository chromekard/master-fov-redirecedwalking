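; Oracle actor with an animated floating static mesh and a controllable audio component.
; From BeginPlay, a timeline restarts whenever it finishes, adding a small local Z offset on each update, interpolated between downward and upward by its Delta track.
; Separate functions let callers swap the sound, stop it, or play it from the start, stopping any current playback first.
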(event `self.ReceiveBeginPlay`
  ;[1 1 1] Anim
  (bind (_direction _delta) (`Timeline|Timeline_0` :!label _label)
    (:`Update`
      (`SceneComponent.K2_AddLocalOffset` (`self.StaticMesh`) (`KismetMathLibrary.MakeVector` 0.0 0.0 (`KismetMathLibrary.Lerp` -0.5 0.5 _delta)) false false))
    (:`Finished`
      (goto _label :!via `PlayFromStart`))))

(fn `PlaySound`
  (if (`AudioComponent.IsPlaying` (`self.Audio`))
    (`AudioComponent.Stop` (`self.Audio`)))
  (`AudioComponent.Play` (`self.Audio`) 0.0)
  (return))

(fn `SetSound`
  (params (NewSound :type "SoundBase Object Reference"))
  (`AudioComponent.SetSound` (`self.Audio`) NewSound)
  (return))

(fn `StopSound`
  (`AudioComponent.Stop` (`self.Audio`))
  (return))

(fn `UserConstructionScript`)