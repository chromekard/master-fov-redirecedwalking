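; BP_Target is a target with a sphere and decal, triggered by cursor hover or pawn overlap while enabled.
; Triggering sets Accepting on BP_Container_GameInstance, fires the Triggered dispatcher, then either expires via a short lifespan or disables itself.
; SetEnabled toggles decal visibility and plays or reverses a timeline driving a disintegrate parameter on dynamic materials.
; The actor pitches -90 degrees on BeginPlay, and SetSphereHeight moves the sphere along local X.
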(event `self.ReceiveBeginPlay`
  (`self.K2_SetActorRotation` (`KismetMathLibrary.MakeRotator` 0.0 -90.0)))

(event `self.Sphere.OnBeginCursorOver`
  (params (TouchedComponent :type "PrimitiveComponent Object Reference"))
  ;[1 1 1] On mouse over
  (if (`self.bEnabled`)
    (bind _asbp_container_game_instance (cast `/Game/Master-fov/Blueprints/GameInstance/BP_Container_GameInstance` (`GameplayStatics.GetGameInstance`)))
    (set `/Game/Master-fov/Blueprints/GameInstance/BP_Container_GameInstance.bAccepting` true _asbp_container_game_instance)
    (`self.EventDispatcher_Triggered`)
    (if (`self.bDestroyOnTrigger`)
      (`self.SetLifeSpan` 0.1)
      (else
        (`self.SetEnabled` false)))))

(event `self.Sphere.OnComponentBeginOverlap`
  (params (OverlappedComponent :type "PrimitiveComponent Object Reference") (OtherActor :type "Actor Object Reference") (OtherComp :type "PrimitiveComponent Object Reference") (OtherBodyIndex :type Integer) (bFromSweep :type Boolean) (SweepResult :type "HitResult Structure (by ref)"))
  ;[1 1 1] Overlapping with pawn class
  (if (`self.bEnabled`)
    (if (`KismetMathLibrary.ClassIsChildOf` (`GameplayStatics.GetObjectClass` OtherActor) "/Script/Engine.Pawn")
      (bind _asbp_container_game_instance (cast `/Game/Master-fov/Blueprints/GameInstance/BP_Container_GameInstance` (`GameplayStatics.GetGameInstance`)))
      (set `/Game/Master-fov/Blueprints/GameInstance/BP_Container_GameInstance.bAccepting` true _asbp_container_game_instance)
      (`self.EventDispatcher_Triggered`)
      (if (`self.bDestroyOnTrigger`)
        (`self.SetLifeSpan` 1.0)
        (else
          (`self.SetEnabled` false))))))

(event `Disintigrate`
  ;[1 1 1] Disintigrate Effect
  (bind _returnvalue (`PrimitiveComponent.CreateDynamicMaterialInstance` (`self.Sphere`) 0 null))
  (bind _returnvalue_2 (`DecalComponent.CreateDynamicMaterialInstance` (`self.Decal`)))
  (bind (_direction _alpha) (`Timeline|Timeline_Disintigrate` :!label _label)
    (:`Update`
      (`MaterialInstanceDynamic.SetScalarParameterValue` _returnvalue "Amount" _alpha)
      (`MaterialInstanceDynamic.SetScalarParameterValue` _returnvalue_2 "Amount" _alpha))))

(event `ReCreate`
  ;[1 1 1] Disintigrate Effect
  (goto _label :!via `ReverseFromEnd`))

(fn `SetEnabled`
  (params (Enabled :type Boolean))
  (set `self.bEnabled` Enabled)
  (`SceneComponent.SetVisibility` (`self.Decal`) Enabled false)
  (if Enabled
    (`self.ReCreate`)
    (else
      (`self.Disintigrate`)))
  (return))

(fn `SetSphereHeight`
  (params (Height :type "Float (double-precision)"))
  (`SceneComponent.K2_SetRelativeLocation` (`self.Sphere`) (`KismetMathLibrary.MakeVector` Height (.y (`SceneComponent.RelativeLocation` (`self.Sphere`))) (.z (`SceneComponent.RelativeLocation` (`self.Sphere`)))) false true)
  (return))

(fn `UserConstructionScript`)