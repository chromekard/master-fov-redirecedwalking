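; BP_BasketBallHoop is a basketball hoop actor that counts scored balls and shows the total on a number widget.
; A Sphere trigger increments Score whenever an overlapping actor's class is exactly BP_Ball_Actor, with no check on direction of travel.
; The Widget component's BP_Number_Widget text is set to Score on BeginPlay and again after each point.
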(event `self.ReceiveBeginPlay`
  (bind _asbp_number_widget (cast `/Game/Master-fov/Widgets/3DWidgets/BP_Number_Widget` (`WidgetComponent.GetUserWidgetObject` (`self.Widget`))))
  (`TextBlock.SetText` (`/Game/Master-fov/Widgets/3DWidgets/BP_Number_Widget.TextBlock_Number` _asbp_number_widget) (`KismetTextLibrary.Conv_IntToText` (`self.Score`))))

(event `self.Sphere.OnComponentBeginOverlap`
  (params (OverlappedComponent :type "PrimitiveComponent Object Reference") (OtherActor :type "Actor Object Reference") (OtherComp :type "PrimitiveComponent Object Reference") (OtherBodyIndex :type Integer) (bFromSweep :type Boolean) (SweepResult :type "HitResult Structure (by ref)"))
  (if (== (`GameplayStatics.GetObjectClass` OtherActor) "/Game/Master-fov/Blueprints/Objects/BP_Ball_Actor.BP_Ball_Actor_C")
    (`/Engine/EditorBlueprintResources/StandardMacros.IncrementInt` (`self.Score`)
      (:`  `
        (bind _asbp_number_widget (cast `/Game/Master-fov/Widgets/3DWidgets/BP_Number_Widget` (`WidgetComponent.GetUserWidgetObject` (`self.Widget`))))
        (`TextBlock.SetText` (`/Game/Master-fov/Widgets/3DWidgets/BP_Number_Widget.TextBlock_Number` _asbp_number_widget) (`KismetTextLibrary.Conv_IntToText` (`self.Score`)))))))

(fn `UserConstructionScript`)