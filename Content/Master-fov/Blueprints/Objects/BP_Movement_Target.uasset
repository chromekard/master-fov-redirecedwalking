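; BP_Movement_Target is a movement goal marker that reacts when a pawn enters its box trigger while enabled.
; On overlap it sets Accepting on the Container game instance, fires the Triggered dispatcher, then either destroys itself after a short lifespan or disables itself.
; SetEnabled tints the sphere green or blue through a dynamic material, and SetHeight moves only the sphere to a given world Z.
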(event `self.ReceiveBeginPlay`
  (bind _returnvalue (`PrimitiveComponent.CreateDynamicMaterialInstance` (`self.Sphere`) 0 null))
  (set `self.DynamicMat` _returnvalue))

(event `self.Box.OnComponentBeginOverlap`
  (params (OverlappedComponent :type "PrimitiveComponent Object Reference") (OtherActor :type "Actor Object Reference") (OtherComp :type "PrimitiveComponent Object Reference") (OtherBodyIndex :type Integer) (bFromSweep :type Boolean) (SweepResult :type "HitResult Structure (by ref)"))
  ;[1 1 1] Overlapping with pawn class
  (if (`self.bEnabled`)
    (if (`KismetMathLibrary.ClassIsChildOf` (`GameplayStatics.GetObjectClass` OtherActor) "/Script/Engine.Pawn")
      (bind _asbp_container_game_instance (cast `/Game/Master-fov/Blueprints/GameInstance/BP_Container_GameInstance` (`GameplayStatics.GetGameInstance`)))
      (set `/Game/Master-fov/Blueprints/GameInstance/BP_Container_GameInstance.bAccepting` true _asbp_container_game_instance)
      (`self.EventDispatcher_Triggered`)
      (if (`self.bDestroyOnTrigger`)
        (`self.SetLifeSpan` 0.1)
        (else
          (`self.SetEnabled` false))))))

(fn `SetEnabled`
  (params (Enabled :type Boolean))
  (bind _output_get (set `self.bEnabled` Enabled))
  (if _output_get
    (`MaterialInstanceDynamic.SetVectorParameterValue` (`self.DynamicMat`) "Color" (struct :`G` 1.0 :`A` 1.0))
    (else
      (`MaterialInstanceDynamic.SetVectorParameterValue` (`self.DynamicMat`) "Color" (struct :`B` 1.0 :`A` 1.0))))
  (return))

(fn `SetHeight`
  (params (z :type "Float (double-precision)"))
  (bind (_returnvalue_x _returnvalue_y) (`KismetMathLibrary.BreakVector` (`SceneComponent.K2_GetComponentLocation` (`self.Sphere`))))
  (`SceneComponent.K2_SetWorldLocation` (`self.Sphere`) (`KismetMathLibrary.MakeVector` _returnvalue_x _returnvalue_y z) false true)
  (return))

(fn `UserConstructionScript`)