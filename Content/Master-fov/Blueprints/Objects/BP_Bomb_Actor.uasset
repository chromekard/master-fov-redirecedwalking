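; BP_Bomb_Actor is a pickup-like sphere that is randomly either a black bomb or a green non-bomb.
; The construction script makes a weighted roll, stores it in Bomb and tints a dynamic material to match.
; Pawn overlap or first hit fires the ExplodePawn event dispatcher with that flag.
; The actor expires almost immediately after a pawn overlap or its first hit on anything.
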(event `self.Sphere1.OnComponentHit`
  (params (HitComponent :type "PrimitiveComponent Object Reference") (OtherActor :type "Actor Object Reference") (OtherComp :type "PrimitiveComponent Object Reference") (NormalImpulse :type "Vector Structure") (Hit :type "HitResult Structure (by ref)"))
  (`/Engine/EditorBlueprintResources/StandardMacros.DoOnce` false
    (:`Completed`
      (if (`KismetMathLibrary.ClassIsChildOf` (`GameplayStatics.GetObjectClass` OtherActor) "/Script/Engine.Pawn")
        (`self.Event_ExplodePawn` (`self.bBomb`)))
      (`self.SetLifeSpan` 0.01))))

(event `self.Sphere.OnComponentBeginOverlap`
  (params (OverlappedComponent :type "PrimitiveComponent Object Reference") (OtherActor :type "Actor Object Reference") (OtherComp :type "PrimitiveComponent Object Reference") (OtherBodyIndex :type Integer) (bFromSweep :type Boolean) (SweepResult :type "HitResult Structure (by ref)"))
  (if (`KismetMathLibrary.ClassIsChildOf` (`GameplayStatics.GetObjectClass` OtherActor) "/Script/Engine.Pawn")
    (`self.Event_ExplodePawn` (`self.bBomb`))
    (`self.SetLifeSpan` 0.01)))

(fn `UserConstructionScript`
  (bind _sphere1 (`self.Sphere1`))
  (bind _sphere1_2 (`self.Sphere1`))
  (bind _output_get (set `self.bBomb` (`KismetMathLibrary.RandomBoolWithWeight` 0.15)))
  (if _output_get
    (bind _returnvalue (`PrimitiveComponent.CreateDynamicMaterialInstance` _sphere1 0 null))
    (`MaterialInstanceDynamic.SetVectorParameterValue` :`self` _returnvalue :`ParameterName` "Color")
    (`PrimitiveComponent.SetMaterial` _sphere1 0 _returnvalue)
    (else
      (bind _returnvalue_2 (`PrimitiveComponent.CreateDynamicMaterialInstance` _sphere1_2 0 null))
      (`MaterialInstanceDynamic.SetVectorParameterValue` _returnvalue_2 "Color" (struct :`G` 1.0 :`A` 1.0))
      (`PrimitiveComponent.SetMaterial` _sphere1_2 0 _returnvalue_2))))