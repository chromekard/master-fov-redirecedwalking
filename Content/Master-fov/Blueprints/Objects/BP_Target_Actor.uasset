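; BP_Target_Actor is a shootable target that disintegrates when hit by a bullet or ball actor, then reforms.
; BeginPlay creates a dynamic material on its Plane, and a hit from BP_Bullet_Actor or BP_Ball_Actor plays a timeline that drives the material's Amount parameter.
; When the timeline finishes, it waits a random few seconds and reverses the timeline from the end to restore the target.
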(event `self.ReceiveBeginPlay`
  (bind _returnvalue (`PrimitiveComponent.CreateDynamicMaterialInstance` (`self.Plane`) 0 null))
  (set `self.DynamicMat` _returnvalue))

(event `self.Plane.OnComponentHit`
  (params (HitComponent :type "PrimitiveComponent Object Reference") (OtherActor :type "Actor Object Reference") (OtherComp :type "PrimitiveComponent Object Reference") (NormalImpulse :type "Vector Structure") (Hit :type "HitResult Structure (by ref)"))
  (bind _returnvalue (`GameplayStatics.GetObjectClass` OtherActor))
  ;[1 1 1] Disintigrate
  (if (or (== _returnvalue "/Game/Master-fov/Blueprints/Objects/BP_Bullet_Actor.BP_Bullet_Actor_C") (== _returnvalue "/Game/Master-fov/Blueprints/Objects/BP_Ball_Actor.BP_Ball_Actor_C"))
    (bind (_direction _alpha) (`Timeline|Timeline_Disintigrate` :!label _label)
      (:`Update`
        (`MaterialInstanceDynamic.SetScalarParameterValue` (`self.DynamicMat`) "Amount" _alpha))
      (:`Finished`
        (`KismetSystemLibrary.Delay` (`KismetMathLibrary.RandomFloatInRange` 3.0 10.0))
        (goto _label :!via `ReverseFromEnd`)))))

(fn `UserConstructionScript`)