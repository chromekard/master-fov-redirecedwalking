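; BP_Cube_Actor is a grabbable physics cube with a randomly colored material.
; Grab turns off physics on the static mesh and attaches the root to a given component while keeping world transform; Release restores physics and detaches.
; The construction script creates a dynamic material instance and sets its Color parameter to random RGB, so each cube gets its own color.
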(event `/Game/Master-fov/Blueprints/Interfaces/BP_Grab_Interface.Grab`
  (params (AttachTo :type "MotionControllerComponent Object Reference"))
  (`PrimitiveComponent.SetSimulatePhysics` (`self.StaticMesh`) false)
  (`SceneComponent.K2_AttachToComponent` (`self.RootComponent`) AttachTo "None" "KeepWorld" "KeepWorld" "KeepWorld" false))

(event `/Game/Master-fov/Blueprints/Interfaces/BP_Grab_Interface.Release`
  (`PrimitiveComponent.SetSimulatePhysics` (`self.StaticMesh`) true)
  (`self.K2_DetachFromActor` "KeepWorld" "KeepWorld" "KeepWorld"))

(fn `UserConstructionScript`
  (bind _staticmesh (`self.StaticMesh`))
  (bind _returnvalue (`PrimitiveComponent.CreateDynamicMaterialInstance` _staticmesh 0 null))
  (`MaterialInstanceDynamic.SetVectorParameterValue` _returnvalue "Color" (make `LinearColor` (`KismetMathLibrary.RandomFloat`) (`KismetMathLibrary.RandomFloat`) (`KismetMathLibrary.RandomFloat`) 1.0))
  (`PrimitiveComponent.SetMaterial` _staticmesh 0 _returnvalue))