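; Ball gun actor that fires BP_Bullet_Actor projectiles from its muzzle and tracks remaining ammo.
; While AutoFire is on, Tick accumulates delta time and calls Fire each time it exceeds Limit.
; Fire spawns a scaled-down bullet, decrements Ammo and updates the count on a widget component, which BeginPlay tints yellow.
; At zero ammo it calls the NoAmmo event to signal a gun drop instead of updating the display.
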(event `self.ReceiveBeginPlay`
  (bind _asbp_number_widget (cast `/Game/Master-fov/Widgets/3DWidgets/BP_Number_Widget` (`WidgetComponent.GetUserWidgetObject` (`self.Ammo_Widget`))))
  (`TextBlock.SetColorAndOpacity` (`/Game/Master-fov/Widgets/3DWidgets/BP_Number_Widget.TextBlock_Number` _asbp_number_widget) (make `SlateColor` (struct :`R` 1.0 :`G` 1.0 :`A` 1.0))))

(event `self.ReceiveTick`
  (params (DeltaSeconds :type "Float (single-precision)"))
  (if (`self.AutoFire`)
    (bind _output_get (set `self.Agrigate` (+ DeltaSeconds (`self.Agrigate`))))
    (if (> _output_get (`self.Limit`))
      (set `self.Agrigate` 0.0)
      (`self.Fire`))))

(fn `Fire`
  (`|SpawnActorFromClass` "/Game/Master-fov/Blueprints/Objects/BP_Bullet_Actor.BP_Bullet_Actor_C" (`KismetMathLibrary.MakeTransform` (.location (`SceneComponent.K2_GetComponentToWorld` (`self.Muzzle`))) (.rotation (`SceneComponent.K2_GetComponentToWorld` (`self.Muzzle`))) (0.1 0.1 0.1)) "AlwaysSpawn" "OverrideRootScale" null null)
  (`/Engine/EditorBlueprintResources/StandardMacros.DecrementInt` (`self.Ammo`)
    (:`  `
      (if (== 0 (`self.Ammo`))
        ;[1 1 1] Drop gun
        (`self.Event_NoAmmo`)
        (else
          (bind _asbp_number_widget (cast `/Game/Master-fov/Widgets/3DWidgets/BP_Number_Widget` (`WidgetComponent.GetUserWidgetObject` (`self.Ammo_Widget`))))
          (`TextBlock.SetText` (`/Game/Master-fov/Widgets/3DWidgets/BP_Number_Widget.TextBlock_Number` _asbp_number_widget) (`KismetTextLibrary.Conv_IntToText` (`self.Ammo`))))))))

(fn `UserConstructionScript`)