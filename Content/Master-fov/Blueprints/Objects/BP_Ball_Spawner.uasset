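; BP_Ball_Spawner is a trigger actor that spawns a ball whenever a pawn overlaps its sphere.
; The overlap event checks for a Pawn subclass, then spawns BP_Ball_Actor at the sphere's world transform with a two-minute lifespan.
; The construction script gives the sphere a dynamic material instance with a random Color, so each spawner gets its own tint.
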(event `self.Sphere.OnComponentBeginOverlap`
  (params (OverlappedComponent :type "PrimitiveComponent Object Reference") (OtherActor :type "Actor Object Reference") (OtherComp :type "PrimitiveComponent Object Reference") (OtherBodyIndex :type Integer) (bFromSweep :type Boolean) (SweepResult :type "HitResult Structure (by ref)"))
  (if (`KismetMathLibrary.ClassIsChildOf` (`GameplayStatics.GetObjectClass` OtherActor) "/Script/Engine.Pawn")
    (bind _returnvalue (`|SpawnActorFromClass` "/Game/Master-fov/Blueprints/Objects/BP_Ball_Actor.BP_Ball_Actor_C" (`SceneComponent.K2_GetComponentToWorld` (`self.Sphere`)) "Undefined" "OverrideRootScale" null null))
    (`self.SetLifeSpan` _returnvalue 120.0)))

(fn `UserConstructionScript`
  (bind _sphere (`self.Sphere`))
  (bind _returnvalue (`PrimitiveComponent.CreateDynamicMaterialInstance` _sphere 0 null))
  (`MaterialInstanceDynamic.SetVectorParameterValue` _returnvalue "Color" (make `LinearColor` (`KismetMathLibrary.RandomFloat`) (`KismetMathLibrary.RandomFloat`) (`KismetMathLibrary.RandomFloat`) 1.0))
  (`PrimitiveComponent.SetMaterial` _sphere 0 _returnvalue))