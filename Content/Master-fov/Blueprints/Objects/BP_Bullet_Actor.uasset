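; BP_Bullet_Actor is an explosive bullet that detonates on its first hit and otherwise expires after a few seconds.
; The sphere's hit event, gated by DoOnce, shortens the lifespan to near zero, fires a RadialForce impulse and spawns an explosion emitter.
; The construction script tints the sphere yellow through a dynamic material instance.
; An explosion sound node exists but is disconnected, so it never plays.
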(event `self.ReceiveBeginPlay`
  (`self.SetLifeSpan` 5.0))

(event `self.Sphere.OnComponentHit`
  (params (HitComponent :type "PrimitiveComponent Object Reference") (OtherActor :type "Actor Object Reference") (OtherComp :type "PrimitiveComponent Object Reference") (NormalImpulse :type "Vector Structure") (Hit :type "HitResult Structure (by ref)"))
  (`/Engine/EditorBlueprintResources/StandardMacros.DoOnce` false
    (:`Completed`
      (`self.SetLifeSpan` 0.01)
      (`RadialForceComponent.FireImpulse` (`self.RadialForce`))
      (`GameplayStatics.SpawnEmitterAtLocation` "/Game/StarterContent/Particles/P_Explosion.P_Explosion" (.location (`self.GetTransform`)) (.rotation (`self.GetTransform`)) (.scale (`self.GetTransform`))))))

(fn `UserConstructionScript`
  (bind _sphere (`self.Sphere`))
  (bind _returnvalue (`PrimitiveComponent.CreateDynamicMaterialInstance` _sphere 0 null))
  (`MaterialInstanceDynamic.SetVectorParameterValue` _returnvalue "Color" (make `LinearColor` 1.0 1.0 0.0 1.0))
  (`PrimitiveComponent.SetMaterial` _sphere 0 _returnvalue))