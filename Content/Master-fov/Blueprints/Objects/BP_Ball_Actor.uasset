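; BP_Ball_Actor is a grabbable physics ball with a random color.
; Grab turns off physics on the sphere and attaches the root to the supplied component, keeping its world transform.
; Release re-enables physics and detaches the actor.
; The construction script creates a dynamic material instance and sets its Color parameter to random RGB values.
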(event `/Game/Master-fov/Blueprints/Interfaces/BP_Grab_Interface.Grab`
  (params (AttachTo :type "MotionControllerComponent Object Reference"))
  (`PrimitiveComponent.SetSimulatePhysics` (`self.Sphere`) false)
  (`SceneComponent.K2_AttachToComponent` (`self.RootComponent`) AttachTo "None" "KeepWorld" "KeepWorld" "KeepWorld" false))

(event `/Game/Master-fov/Blueprints/Interfaces/BP_Grab_Interface.Release`
  (`PrimitiveComponent.SetSimulatePhysics` (`self.Sphere`) true)
  (`self.K2_DetachFromActor` "KeepWorld" "KeepWorld" "KeepWorld"))

(fn `UserConstructionScript`
  (bind _sphere (`self.Sphere`))
  (bind _returnvalue (`PrimitiveComponent.CreateDynamicMaterialInstance` _sphere 0 null))
  (`MaterialInstanceDynamic.SetVectorParameterValue` _returnvalue "Color" (make `LinearColor` (`KismetMathLibrary.RandomFloat`) (`KismetMathLibrary.RandomFloat`) (`KismetMathLibrary.RandomFloat`) 1.0))
  (`PrimitiveComponent.SetMaterial` _sphere 0 _returnvalue))